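; Pappzombie is a Salon prop that acts as a one-time scare for the NoEndHouseCharacter.
; The first time the character enters its Box trigger, it lowers the character's Sanity and plays a placeholder skeletal animation once.
; HudInfo appears after a short delay on that first trigger, immediately on later entries, and hides when the character leaves the box.
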(event `self.Box.OnComponentBeginOverlap`
  (params (OverlappedComponent :type "PrimitiveComponent Object Reference") (OtherActor :type "Actor Object Reference") (OtherComp :type "PrimitiveComponent Object Reference") (OtherBodyIndex :type Integer) (bFromSweep :type Boolean) (SweepResult :type "HitResult Structure (by ref)"))
  (bind _asno_end_house_character (cast `NoEndHouseCharacter` OtherActor))
  (if (not (`self.played`))
    (set `self.played` true)
    (`NoEndHouseCharacter.SetSanity` _asno_end_house_character (- (`NoEndHouseCharacter.Sanity` _asno_end_house_character) 35.0))
    (`SkeletalMeshComponent.PlayAnimation` (`self.SkeletalMeshComponent`) "/Game/Props/Salon/PappZombie/Pappzombie_placeholder_Anim.Pappzombie_placeholder_Anim" false)
    (`KismetSystemLibrary.Delay` 0.5))
  (`SceneComponent.SetVisibility` (`self.Hud Info`) true false))

(event `self.Box.OnComponentEndOverlap`
  (params (OverlappedComponent :type "PrimitiveComponent Object Reference") (OtherActor :type "Actor Object Reference") (OtherComp :type "PrimitiveComponent Object Reference") (OtherBodyIndex :type Integer))
  (cast `NoEndHouseCharacter` OtherActor)
  (`SceneComponent.SetVisibility` (`self.Hud Info`) false false))

(fn `UserConstructionScript`)