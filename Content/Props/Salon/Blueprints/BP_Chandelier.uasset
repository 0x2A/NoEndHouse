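; Salon chandelier prop Blueprint whose three lights and glowing material can be dimmed or brightened together.
; BeginPlay caches the base intensities of two point lights and a spot light, and creates a dynamic instance of the Chandelier_Light material.
; SetLightIntensity scales the lights by those cached values and drives the material's Brightness parameter in proportion.
; PointLight1 reuses the spot light's cached base, leaving its own unused.
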(event `self.ReceiveBeginPlay`
  (set `self.BaseLightIntensity` (`|MakeArray` (`LightComponentBase.Intensity` (`self.PointLight`)) (`LightComponentBase.Intensity` (`self.SpotLight`)) (`LightComponentBase.Intensity` (`self.PointLight1`))))
  (bind _returnvalue (`PrimitiveComponent.CreateDynamicMaterialInstance` (`self.StaticMeshComponent`) 0 "/Game/Props/Salon/Lights/Chandelier_Light.Chandelier_Light"))
  (set `self.LightMaterial` _returnvalue))

(fn `SetLightIntensity`
  (params (Intensity :type "Float (double-precision)"))
  (bind _baselightintensity (`self.BaseLightIntensity`))
  (`LightComponent.SetIntensity` (`self.PointLight`) (* Intensity (`KismetArrayLibrary.Array_Get` _baselightintensity)))
  (`LightComponent.SetIntensity` (`self.SpotLight`) (* Intensity (`KismetArrayLibrary.Array_Get` _baselightintensity 1)))
  (`LightComponent.SetIntensity` (`self.PointLight1`) (* Intensity (`KismetArrayLibrary.Array_Get` _baselightintensity 1)))
  (`MaterialInstanceDynamic.SetScalarParameterValue` (`self.LightMaterial`) "Brightness" (* Intensity 3.5)))

(fn `UserConstructionScript`)