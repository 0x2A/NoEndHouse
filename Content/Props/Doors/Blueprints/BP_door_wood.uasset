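; Wooden door prop that the NoEndHouseCharacter opens and closes with the Use input, unlocking if the character carries its key.
; Overlap checks the inventory for KeyId, enables input and shows HudMsg; leaving reverses the input and message.
; DoorTimeline drives mesh yaw forward or backward from a start time set by HalfOpenValue.
; Sounds mark opening start, closing finish and locked attempts; PlayDoorSound is defined but uncalled here.
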(event `self.ReceiveBeginPlay`
  (`TimelineComponent.SetNewTime` (`self.DoorTimeline`) (`self.HalfOpenValue`)))

(event `self.ReceiveActorBeginOverlap`
  (params (OtherActor :type "Actor Object Reference"))
  (bind _asno_end_house_character (cast `NoEndHouseCharacter` OtherActor))
  (`|ExecutionSequence`
    (:`then_0`
      (if (`self.Locked`)
        (bind _returnvalue (`InventoryInterfaceBPFunctionLib.CheckInventory` _asno_end_house_character (`self.KeyId`)))
        (set `self.Locked` (not _returnvalue))))
    (:`then_1`
      (`self.EnableInput` (`NoEndHouseCharacter.PlayerController` _asno_end_house_character))
      (`SceneComponent.SetVisibility` (`self.HudMsg`) true true))))

(event `self.ReceiveActorEndOverlap`
  (params (OtherActor :type "Actor Object Reference"))
  (bind _asno_end_house_character (cast `NoEndHouseCharacter` OtherActor))
  (`self.DisableInput` (`NoEndHouseCharacter.PlayerController` _asno_end_house_character))
  (`SceneComponent.SetVisibility` (`self.HudMsg`) false true))

(event `DoorOpening`
  (bind (_direction _doorrot _time) (`Timeline|DoorTimeline` :!label _label)
    (:`Update`
      (`SceneComponent.K2_SetRelativeRotation` (`self.DoorMesh`) (`KismetMathLibrary.MakeRotator` 0.0 0.0 _doorrot) false false)
      (if (and (<= _time 0.05) (`|EnumEquality` _direction "Forward"))
        (`AudioComponent.Play` (`self.OpeningDoor`) 0.0)))
    (:`Finished`
      (switch `ETimelineDirection` _direction
        (:`Backward`
          (`AudioComponent.Play` (`self.ClosingDoor`) 0.0))))))

(event `DoorClosing`
  (goto _label :!via `Reverse`))

(event `InputAction|Use`
  (params (Key :type "Key Structure" :default "AnyKey"))
  (:`Pressed`
    (if (`self.DoorClosed`)
      (`self.OpenDoor`)
      (else
        (`self.CloseDoor`)))))

(fn `CloseDoor`
  (set `self.DoorClosed` true)
  (`self.DoorClosing`))

(fn `OpenDoor`
  (bind _lockedsound (`self.LockedSound`))
  (if (`self.Locked`)
    (if (not (`AudioComponent.IsPlaying` _lockedsound))
      (`AudioComponent.Play` _lockedsound 0.0))
    (else
      (set `self.DoorClosed` false)
      (`self.DoorOpening`))))

(fn `PlayDoorSound`
  (params (time :type "Float (double-precision)") (Close :type Boolean))
  (bind _openingdoor (`self.OpeningDoor`))
  (bind _openingdoor_2 (`self.OpeningDoor`))
  (bind _closingdoor (`self.ClosingDoor`))
  (bind _closingdoor_2 (`self.ClosingDoor`))
  (if (`self.Locked`)
    _
    (elif Close
      (if (`AudioComponent.IsPlaying` _openingdoor)
        (`AudioComponent.Stop` _openingdoor))
      (if (not (`AudioComponent.IsPlaying` _closingdoor))
        (`AudioComponent.Play` _closingdoor time))
      (else
        (if (`AudioComponent.IsPlaying` _closingdoor_2)
          (`AudioComponent.Stop` _closingdoor_2))
        (if (not (`AudioComponent.IsPlaying` _openingdoor_2))
          (`AudioComponent.Play` _openingdoor_2 time))))))

(fn `UserConstructionScript`)