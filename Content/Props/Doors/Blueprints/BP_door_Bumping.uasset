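; A door prop that rattles and bumps once when the player character walks into its trigger box.
; The overlap plays a rattle sound and a timeline that swings the mesh's yaw, then destroys the box so it cannot repeat.
; Standard door logic remains (open/close timeline, locked sound, key check, HUD prompt), but the interaction and unlock paths are disconnected and PlayDoorSound does nothing.
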(event `self.ReceiveBeginPlay`
  (`TimelineComponent.SetNewTime` (`self.DoorTimeline`) (`self.HalfOpenValue`)))

(event `self.ReceiveActorEndOverlap`
  (params (OtherActor :type "Actor Object Reference"))
  (bind _asno_end_house_character (cast `NoEndHouseCharacter` OtherActor))
  (`self.DisableInput` (`NoEndHouseCharacter.PlayerController` _asno_end_house_character))
  (`SceneComponent.SetVisibility` (`self.HudMsg`) false true))

(event `DoorOpening`
  (bind (_direction _doorrot _time) (`Timeline|DoorTimeline` :!label _label)
    (:`Update`
      (`SceneComponent.K2_SetRelativeRotation` (`self.DoorMesh`) (`KismetMathLibrary.MakeRotator` 0.0 0.0 _doorrot) false false)
      (if (and (<= _time 0.05) false)
        _))
    (:`Finished`
      (switch `ETimelineDirection` _direction))))

(event `DoorClosing`
  (goto _label :!via `Reverse`))

(event `self.Box.OnComponentBeginOverlap`
  (params (OverlappedComponent :type "PrimitiveComponent Object Reference") (OtherActor :type "Actor Object Reference") (OtherComp :type "PrimitiveComponent Object Reference") (OtherBodyIndex :type Integer) (bFromSweep :type Boolean) (SweepResult :type "HitResult Structure (by ref)"))
  (cast `NoEndHouseCharacter` OtherActor)
  (set `PrimitiveComponent.bGenerateOverlapEvents` false (`self.Box`))
  (`AudioComponent.Play` (`self.door_rattle`) 0.0)
  (bind (_direction _rotation) (`Timeline|DoorBumping`)
    (:`Update`
      (`SceneComponent.K2_SetRelativeRotation` (`self.DoorMesh`) (`KismetMathLibrary.MakeRotator` 0.0 0.0 _rotation) false false))
    (:`Finished`
      (`ActorComponent.K2_DestroyComponent` (`self.Box`)))))

(fn `CloseDoor`
  (set `self.DoorClosed` true)
  (`self.DoorClosing`))

(fn `OpenDoor`
  (bind _lockedsound (`self.LockedSound`))
  (if (`self.Locked`)
    (if (not (`AudioComponent.IsPlaying` _lockedsound))
      (`AudioComponent.Play` _lockedsound 0.0))
    (else
      (set `self.DoorClosed` false)
      (`self.DoorOpening`))))

(fn `PlayDoorSound`
  (params (time :type "Float (double-precision)") (Close :type Boolean))
  (if (`self.Locked`)
    _
    (elif Close
      (if false
        _
        (elif false
          _))
      (elif false
        _
        (elif false
          _)))))

(fn `UserConstructionScript`)