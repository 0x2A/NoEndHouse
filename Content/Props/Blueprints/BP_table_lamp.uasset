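; Table lamp prop Blueprint whose light brightness can be scaled as a whole.
; On BeginPlay it caches the starting intensities of its two point lights.
; SetLightIntensity then multiplies each cached base value by the given factor, so both lights keep their relative brightness.
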(event `self.ReceiveBeginPlay`
  (set `self.BaseLightIntensity` (`|MakeArray` (`LightComponentBase.Intensity` (`self.PointLight`)) (`LightComponentBase.Intensity` (`self.PointLight1`)))))

(fn `SetLightIntensity`
  (params (Intensity :type "Float (double-precision)"))
  (bind _baselightintensity (`self.BaseLightIntensity`))
  (`LightComponent.SetIntensity` (`self.PointLight`) (* Intensity (`KismetArrayLibrary.Array_Get` _baselightintensity)))
  (`LightComponent.SetIntensity` (`self.PointLight1`) (* Intensity (`KismetArrayLibrary.Array_Get` _baselightintensity 1))))

(fn `UserConstructionScript`)