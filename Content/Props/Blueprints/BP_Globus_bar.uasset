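; BP_Globus_bar is an interactable globe bar prop, not pickable, whose top swings open and closed.
; Each interaction toggles IsOpen and plays or reverses the GlobusRotation timeline, which drives the relative roll of GlobusBarTop.
; RotFinished blocks new interactions until the timeline finishes.
; On BeginPlay, an IsOpen instance snaps its top to a fixed open rotation.
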(event `self.ReceiveBeginPlay`
  (if (`self.isOpen`)
    (`SceneComponent.K2_SetRelativeRotation` (`self.Globus_Bar_Top`) (struct :`Roll` 89.5) false false)))

(event `self.BeginInteraction`
  (bind _isopen (`self.isOpen`))
  (if (`self.RotFinished`)
    (set `self.RotFinished` false)
    (set `self.isOpen` (not _isopen))
    (if _isopen
      (bind (_direction _rotation) (`Timeline|GlobusRotation` :!label _label)
        (:`Update`
          (`SceneComponent.K2_SetRelativeRotation` (`self.Globus_Bar_Top`) (`KismetMathLibrary.MakeRotator` _rotation) false false))
        (:`Finished`
          (set `self.RotFinished` true)))
      (else
        (goto _label :!via `Reverse`)))))

(fn `AllowInteraction`
  (returns (ReturnValue :type Boolean))
  (return true))

(fn `CanPickup`
  (returns (ReturnValue :type Boolean))
  (return false))

(fn `UserConstructionScript`)