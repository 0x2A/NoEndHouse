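; Book shelf prop that fills a row along local X with book instances in its construction script, up to the horizontal length of EndPoint.
; A random stream varies each book's thickness, height, depth offset and slight tilt, with a random branch adding extra Steps spacing between some books.
; All books share one InstancedStaticMesh, scaled by BookHeightScale, with a dynamic material chosen by DesignNumber and tinted by cover color and dirt parameters.
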(fn `UserConstructionScript`
  (bind _randomstream (`self.RandomStream`))
  (bind _instancedstaticmesh (`self.InstancedStaticMesh`))
  (bind _instancedstaticmesh_2 (`self.InstancedStaticMesh`))
  (bind _instancedstaticmesh_3 (`self.InstancedStaticMesh`))
  (bind _randomrotatetemp (`self.RandomRotateTemp`))
  (bind _returnvalue (`KismetMathLibrary.RandomFloatInRangeFromStream` -2.0 2.0 _randomstream))
  (bind _returnvalue_2 (`KismetMathLibrary.RandomFloatInRangeFromStream` 0.97 1.0 _randomstream))
  (bind _returnvalue_3 (`KismetMathLibrary.RandomFloatInRangeFromStream` -5.0 5.0 _randomstream))
  (bind _returnvalue_4 (+ (`self.BookLengthSum`) (`self.BookThicnessTemp`)))
  (bind _returnvalue_5 (+ (`self.BookLengthSum`) (`self.BookThicnessTemp`) (`self.Steps`)))
  (bind _returnvalue_6 (`KismetMathLibrary.MakeTransform` (`KismetMathLibrary.MakeVector` _returnvalue_4 _returnvalue_3) (`KismetMathLibrary.MakeRotator` 0.0 _returnvalue) (`KismetMathLibrary.MakeVector` (`self.RandomScaleTemp`) 1.0 _returnvalue_2)))
  (`|ExecutionSequence`
    (:`then_0`
      ;[1 1 1] Create the first mesh of the book
      (`/Engine/EditorBlueprintResources/StandardMacros.DoOnce` false
        (:`Completed`
          (`StaticMeshComponent.SetStaticMesh` _instancedstaticmesh_3 (`self.Mesh to Spawn`))
          (`InstancedStaticMeshComponent.AddInstance` _instancedstaticmesh_3 (`KismetMathLibrary.MakeTransform` (0.0 0.0 0.0) (struct) (1.0 1.0 1.0)))
          (`SceneComponent.SetWorldScale3D` _instancedstaticmesh_3 (`KismetMathLibrary.MakeVector` 1.0 1.0 (`self.Book Height Scale`)))
          (set `self.BookThicnessTemp` (`self.Book Thickness`))
          ;[1 1 1] Change Dynamic Material
          (`PrimitiveComponent.CreateDynamicMaterialInstance` _instancedstaticmesh_2 0 (`|GetArrayItem` (`self.MatVarious`) (`self.Design Number`)) :!label _label)
          (`MeshComponent.SetVectorParameterValueOnMaterials` _instancedstaticmesh_2 "CoverColor" (`KismetMathLibrary.Conv_LinearColorToVector` (`self.CoverColor`)))
          (`MeshComponent.SetScalarParameterValueOnMaterials` _instancedstaticmesh_2 "DirtColorControl" (`self.Color Control`)))))
    (:`then_1`
      (while (> (`KismetMathLibrary.VSize` (* (`self.End Point`) (1.0 1.0 0.0))) (+ (`self.BookLengthSum`) 15.0))
        (set `self.RandomScaleTemp` (`KismetMathLibrary.RandomFloatInRangeFromStream` 0.5 1.7 _randomstream))
        (set `self.RandomRotateTemp` _returnvalue)
        (`StaticMeshComponent.SetStaticMesh` _instancedstaticmesh (`self.Mesh to Spawn`))
        (if (> _randomrotatetemp 1.5)
          (set `self.TransformTemp` (`KismetMathLibrary.MakeTransform` (`KismetMathLibrary.MakeVector` _returnvalue_5 _returnvalue_3) (`KismetMathLibrary.MakeRotator` 0.0 _returnvalue) (`KismetMathLibrary.MakeVector` (`self.RandomScaleTemp`) 1.0 _returnvalue_2)))
          (set `self.BookLengthSum` _returnvalue_5)
          (set `self.BookThicnessTemp` (* (`self.RandomScaleTemp`) (`self.Book Thickness`)) :!label _label_2)
          (elif (< -1.5 _randomrotatetemp)
            (set `self.TransformTemp` _returnvalue_6)
            (set `self.BookLengthSum` _returnvalue_4)
            (set `self.BookThicnessTemp` (+ (* (`self.RandomScaleTemp`) (`self.Book Thickness`)) (`self.Steps`)))
            (else
              (set `self.TransformTemp` _returnvalue_6)
              (set `self.BookLengthSum` _returnvalue_4)
              (goto _label_2))))
        (`InstancedStaticMeshComponent.AddInstance` _instancedstaticmesh (`self.TransformTemp`))
        (goto _label)))))