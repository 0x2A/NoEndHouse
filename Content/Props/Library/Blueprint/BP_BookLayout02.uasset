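; BP_BookLayout02 is a prop Blueprint that procedurally lays out a row of books as instanced static meshes.
; Its construction script places a first book, then adds more along local X until their summed length nears the EndPoint's horizontal distance.
; A random stream varies each book's thickness, height and depth offset, while tilt accumulates from StartAngle using EndAngle plus jitter.
; A dynamic material selected by DesignNumber sets cover color and dirt.
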(fn `UserConstructionScript`
  (bind _randomstream (`self.RandomStream`))
  (bind _instancedstaticmesh (`self.InstancedStaticMesh`))
  (bind _instancedstaticmesh_2 (`self.InstancedStaticMesh`))
  (bind _instancedstaticmesh_3 (`self.InstancedStaticMesh`))
  (bind _returnvalue (+ (`self.BookLengthSum`) (`self.BookThicnessTemp`)))
  (`|ExecutionSequence`
    (:`then_0`
      ;[1 1 1] Create the first mesh of the book
      (`/Engine/EditorBlueprintResources/StandardMacros.DoOnce` false
        (:`Completed`
          (`StaticMeshComponent.SetStaticMesh` _instancedstaticmesh_3 (`self.Mesh to Spawn`))
          (`InstancedStaticMeshComponent.AddInstance` _instancedstaticmesh_3 (`KismetMathLibrary.MakeTransform` (0.0 0.0 0.0) (`KismetMathLibrary.MakeRotator` 0.0 (`self.StartAngle`)) (`KismetMathLibrary.MakeVector` 1.0 1.0 (`self.Book Height Scale`))))
          (set `self.BookThicnessTemp` 13.0)
          (set `self.TempAngle` (`self.StartAngle`))
          (set `self.count` 2.0)
          ;[1 1 1] Change Dynamic Material
          (`PrimitiveComponent.CreateDynamicMaterialInstance` _instancedstaticmesh_2 0 (`|GetArrayItem` (`self.MatVarious`) (`self.Design Number`)) :!label _label)
          (`MeshComponent.SetVectorParameterValueOnMaterials` _instancedstaticmesh_2 "CoverColor" (`KismetMathLibrary.Conv_LinearColorToVector` (`self.CoverColor`)))
          (`MeshComponent.SetScalarParameterValueOnMaterials` _instancedstaticmesh_2 "DirtColorControl" (`self.Color Control`)))))
    (:`then_1`
      (while (> (`KismetMathLibrary.VSize` (* (`self.End Point`) (1.0 1.0 0.0))) (+ (`self.BookLengthSum`) 15.0))
        (set `self.RandomScaleTemp` (`KismetMathLibrary.RandomFloatInRangeFromStream` 0.5 1.3 _randomstream))
        (`StaticMeshComponent.SetStaticMesh` _instancedstaticmesh (`self.Mesh to Spawn`))
        (bind _output_get (set `self.TempAngle` (+ (+ (`self.TempAngle`) (/ (`self.EndAngle`) 10.0)) (`KismetMathLibrary.RandomFloatInRangeFromStream` -1.0 1.0 _randomstream))))
        (set `self.TransformTemp` (`KismetMathLibrary.MakeTransform` (`KismetMathLibrary.MakeVector` _returnvalue (`KismetMathLibrary.RandomFloatInRangeFromStream` -5.0 5.0 _randomstream)) (`KismetMathLibrary.MakeRotator` 0.0 _output_get) (`KismetMathLibrary.MakeVector` (`self.RandomScaleTemp`) 1.0 (* (`KismetMathLibrary.RandomFloatInRangeFromStream` 0.95 1.0 _randomstream) (`self.Book Height Scale`)))))
        (set `self.BookLengthSum` _returnvalue)
        (set `self.BookThicnessTemp` (+ (* (`self.RandomScaleTemp`) (`self.Book Thickness`)) (* (`self.Steps`) (`self.count`))))
        (set `self.count` (+ (`self.count`) 1.0))
        (`InstancedStaticMeshComponent.AddInstance` _instancedstaticmesh (`self.TransformTemp`))
        (goto _label)))))