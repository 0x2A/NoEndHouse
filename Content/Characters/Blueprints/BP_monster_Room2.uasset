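; BP_monster_Room2 is the Room 2 monster encounter, which the player dispels by blinking.
; On BeginPlay it binds to the player character's end-blink delegate and, after a short delay for Chandelier setup, turns the chandelier off.
; Entering its one-shot trigger box freezes the player and shows a HUD hint.
; A long enough blink afterwards hides the monster, restores movement and switches light from lamp to chandelier.
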(event `self.ReceiveBeginPlay`
  (bind _asno_end_house_character (cast `NoEndHouseCharacter` (`GameplayStatics.GetPlayerCharacter` 0)))
  (add `NoEndHouseCharacter.OnEndBlinkDelegate` _asno_end_house_character (delegate `OnEndBlink`))
  (`KismetSystemLibrary.Delay` 1.0) ; Need delay because beginEdit of Chandelier might not have called yet
  (`/Game/Props/Salon/Blueprints/BP_Chandelier.SetLightIntensity` (`self.Chandelier`) 0.0))

(event `OnEndBlink`
  (params (BlinkTime :type "Float (double-precision)"))
  (if (and (> BlinkTime 0.33) (`self.EnteredTriggerBox`))
    (`/Game/Props/Blueprints/BP_table_lamp.SetLightIntensity` (`self.Lamp_Light`) 0.0)
    (set `NoEndHouseCharacter.bCanMove` true (stale `self.ReceiveBeginPlay` _asno_end_house_character))
    (`SceneComponent.SetVisibility` (`self.SkeletalMesh`) false true)
    (`/Game/Props/Salon/Blueprints/BP_Chandelier.SetLightIntensity` (`self.Chandelier`) 1.0)))

(event `self.TriggerBox.OnComponentBeginOverlap`
  (params (OverlappedComponent :type "PrimitiveComponent Object Reference") (OtherActor :type "Actor Object Reference") (OtherComp :type "PrimitiveComponent Object Reference") (OtherBodyIndex :type Integer) (bFromSweep :type Boolean) (SweepResult :type "HitResult Structure (by ref)"))
  (bind _asno_end_house_character (cast `NoEndHouseCharacter` OtherActor))
  (set `PrimitiveComponent.bGenerateOverlapEvents` false (`self.TriggerBox`))
  (set `self.EnteredTriggerBox` true)
  (set `NoEndHouseCharacter.bCanMove` false _asno_end_house_character)
  (`SceneComponent.SetVisibility` (`self.HUD_Hint`) true false))

(fn `UserConstructionScript`)