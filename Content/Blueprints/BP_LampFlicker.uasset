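; BP_LampFlicker is a one-shot trigger that flickers assigned lamps with sound when a Character enters its box, leaving them almost dark.
; BeginPlay caches the first light component and original intensity of each TargetLight actor.
; On overlap, it plays the audio and a timeline whose curve scales each cached intensity every update.
; When the timeline finishes, the actor destroys itself and sets the lights to a near-zero fraction of their original intensity.
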(event `self.ReceiveBeginPlay`
  (for (_array_element _array_index) (`self.TargetLight`)
    (bind _returnvalue (`self.K2_GetComponentsByClass` _array_element "/Script/Engine.LightComponent"))
    (if (> (`KismetArrayLibrary.Array_Length` _returnvalue) 0)
      (bind _item (`KismetArrayLibrary.Array_Get` _returnvalue))
      (`KismetArrayLibrary.Array_Insert` (`self.TargetLightComp`) _item _array_index)
      (`KismetArrayLibrary.Array_Insert` (`self.LightIntensity`) (`LightComponentBase.Intensity` _item) _array_index))))

(event `self.Box.OnComponentBeginOverlap`
  (params (OtherActor :type "Actor Object Reference") (OtherComp :type "PrimitiveComponent Object Reference") (OtherBodyIndex :type Integer) (bFromSweep :type Boolean) (SweepResult :type "HitResult Structure (by ref)"))
  (cast `Character` OtherActor)
  (if (> (`KismetArrayLibrary.Array_Length` (`self.TargetLightComp`)) 0)
    (`AudioComponent.Play` (`self.Audio`) 0.0)
    (bind (_direction _lightintensity) (`Timeline|Timeline_LightIntensity`)
      (:`Update`
        (set `self.newLightInt` _lightintensity))
      (:`Finished`
        (set `self.newLightInt` 0.01)
        (`self.K2_DestroyActor`)))
    (for (_array_element _array_index) (`self.TargetLightComp`)
      (`LightComponent.SetIntensity` _array_element (* (`self.newLightInt`) (`KismetArrayLibrary.Array_Get` (`self.LightIntensity`) _array_index))))))

(fn `UserConstructionScript`)