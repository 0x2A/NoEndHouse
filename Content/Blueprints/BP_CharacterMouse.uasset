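; BP_CharacterMouse is a mouse character that can always be picked up and reacts to being observed.
; When observation begins, it disables movement and turns on physics simulation for its capsule.
; When observation ends, it turns physics off, resets the capsule upright while keeping its yaw, and re-enables movement.
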(event `self.ReceiveTick`
  (params (DeltaSeconds :type "Float (single-precision)")))

(event `self.BeginObservation`
  (`self.DisableMovement`)
  (`PrimitiveComponent.SetSimulatePhysics` (`self.CapsuleComponent`) true))

(event `self.EndObservation`
  (bind _capsulecomponent (`self.CapsuleComponent`))
  (`PrimitiveComponent.SetSimulatePhysics` _capsulecomponent false)
  (`SceneComponent.K2_SetWorldRotation` _capsulecomponent (`KismetMathLibrary.MakeRotator` 0.0 0.0 (.yaw (`SceneComponent.K2_GetComponentRotation` _capsulecomponent))) false false)
  (`self.EnableMovement`))

(fn `CanPickup`
  (returns (ReturnValue :type Boolean))
  (return true))

(fn `UserConstructionScript`)