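; NEHKey1 is a key pickup Blueprint that dissolves away when picked up, then destroys itself.
; OnPickUp plays a timeline that writes its value into the DissolveAmount scalar parameter of each stored material instance, and destroys the actor when the timeline finishes.
; CanPickup allows pickup while PickedUp is false, though this file never sets that flag or fills the material instance array.
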(event `self.OnPickUp`
  (bind _materialinstances (`self.MaterialInstances`))
  (bind (_direction _dissolvevlaue) (`Timeline|Timeline_Dissolve`)
    (:`Update`
      (for _index (range (+ (`KismetArrayLibrary.Array_Length` _materialinstances) 1))
        (`MaterialInstanceDynamic.SetScalarParameterValue` (`KismetArrayLibrary.Array_Get` _materialinstances _index) "DissolveAmount" _dissolvevlaue)))
    (:`Finished`
      (`self.K2_DestroyActor`))))

(fn `CanPickup`
  (returns (ReturnValue :type Boolean))
  (return (not (`self.bPickedUp`))))

(fn `UserConstructionScript`)