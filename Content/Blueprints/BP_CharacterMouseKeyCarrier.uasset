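; Mouse character key carrier that gives up its key when rotated far enough while being observed.
; ObservingChangedRotation dots the new rotation's up vector with an unnormalized X/-Z diagonal, accepting either sign above a threshold.
; The first match sets a one-shot flag and, after a short delay, plays a timeline that cumulatively offsets the Key along local X.
; It also immediately calls PickUp on the Key's NEHKey1_Blueprint child actor as the slide starts.
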(event `self.ObservingChangedRotation`
  (params (newRotation :type "Rotator Structure"))
  (if (and (>= (`KismetMathLibrary.Abs` (`KismetMathLibrary.Dot_VectorVector` (`KismetMathLibrary.GetUpVector` newRotation) (`KismetMathLibrary.MakeVector` 1.0 0.0 -1.0))) 0.925) (not (`self.PickedUp`)))
    (set `self.PickedUp` true)
    (`KismetSystemLibrary.Delay` 0.5)
    (`|ExecutionSequence`
      (:`then_0`
        (bind (_direction _positionoffset) (`Timeline|Timeline_0`)
          (:`Update`
            (`SceneComponent.K2_AddLocalOffset` (`self.Key`) (`KismetMathLibrary.MakeVector` _positionoffset) false false))))
      (:`then_1`
        (bind _asnehkey_1_blueprint (cast `/Game/Blueprints/NEHKey1_Blueprint` (`ChildActorComponent.ChildActor` (`self.Key`))))
        (`NEHKey.PickUp` _asnehkey_1_blueprint)))))

(fn `UserConstructionScript`
  (`parent.UserConstructionScript`))